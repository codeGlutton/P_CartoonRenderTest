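; Test character Blueprint that repeatedly runs a mesh component lookup every Tick, apparently to compare lookup methods.
; A loop calls FindMeshCompByC and passes the result and index to NewFunction on each iteration.
; NewFunction joins both as text into NewVar, overwriting it each call.
; Two alternative lookups, FindMeshCompByBPNative and GetComponentByClass for SkeletalMeshComponent, sit disconnected and never run.
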(event `self.ReceiveTick`
  (params (DeltaSeconds :type "Float (single-precision)"))
  (for _index (range 101)
    (set `self.Index` _index)
    (bind _returnvalue (`MyBlueprintFunctionLibrary.FindMeshCompByC` self))
    (`self.NewFunction` _returnvalue (`self.Index`))))

(event `NewFunction`
  (params (InObj :type "Object Object Reference") (InInt :type Integer))
  (set `self.NewVar` (`KismetStringLibrary.Concat_StrStr` (`KismetStringLibrary.Conv_ObjectToString` InObj) (`KismetStringLibrary.Conv_IntToString` InInt))))

(fn `UserConstructionScript`)